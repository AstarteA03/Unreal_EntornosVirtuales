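; BP_FinalDoor is a door actor that opens once every collectable item in the level has been collected.
; On BeginPlay it counts all BP_CollectableItem actors, opening immediately if there are none.
; Its ItemCollected event decrements that count and calls OpenDoor at zero.
; Opening destroys the door and plays a music cue at the world origin.
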(event `self.ReceiveBeginPlay`
  (bind _outactors (`GameplayStatics.GetAllActorsOfClass` "/Game/IA/GamePlayComponents/BP_CollectableItem.BP_CollectableItem_C"))
  (bind _output_get (set `self.RemainingCollectableItem` (`KismetArrayLibrary.Array_Length` _outactors)))
  (if (== _output_get 0)
    (`self.OpenDoor`)))

(event `OpenDoor`
  (`self.K2_DestroyActor`)
  (`GameplayStatics.PlaySoundAtLocation` "/Game/StarterContent/Audio/Starter_Music_Cue.Starter_Music_Cue" (0.0 0.0 0.0) (struct) 1.0 1.0 0.0 null null null null))

(event `ItemCollected`
  (bind _result (`/Engine/EditorBlueprintResources/StandardMacros.DecrementInt` (`self.RemainingCollectableItem`))
    (:`  `
      (if (== _result 0)
        (`self.OpenDoor`)))))

(fn `UserConstructionScript`)